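; Train actor that travels along the spline of a referenced track, starting on BeginPlay when it is flagged active.
; MoveTrain plays the TrainMover timeline at a rate derived from Duration, beginning at a configurable time offset.
; Each update maps the timeline alpha to distance along the spline and applies that point's world location and rotation to the actor.
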(event Custom|MoveTrain
  (bind _trackref (Variables|Default|GetTrackRef))
  (bind _usefulspline (Variables|/Game/Blueprints/Track.Track_C|GetUsefulSpline _trackref))
  (Components|Timeline|SetPlayRate (Variables|Default|GetTrainMover) (/ 1.0 (Variables|Default|GetDuration)))
  (Components|Timeline|SetNewTime (Variables|Default|GetTrainMover) (Variables|Default|GetTrainStartOffset))
  (bind _alpha (Timeline|TrainMover Play)
    (:Update
      (Variables|Default|SetAlpha _alpha)
      (Transformation|SetActorLocationAndRotation (Spline|GetLocationatDistanceAlongSpline _usefulspline (Math|Float|Lerp 0.0 (Spline|GetSplineLength _usefulspline) (Variables|Default|GetAlpha)) "World") (Spline|GetRotationatDistanceAlongSpline _usefulspline (Math|Float|Lerp 0.0 (Spline|GetSplineLength _usefulspline) (Variables|Default|GetAlpha)) "World")))))

(event EventBeginPlay
  (if (Variables|Default|GetActiveTrain)
    (CallFunction|MoveTrain)))

(fn ConstructionScript)